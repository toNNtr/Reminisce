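; BP_Memorable is a one-shot interactable actor that swaps streaming levels when used.
; Interact runs DoAction, which, if enabled, fires the LoadLevels dispatcher, then disables the actor and switches its material.
; The bound handler uses an index-driven loop over latent stream calls, loading each listed level in sequence before unloading the others.
; The construction script applies the configurable mesh, enabled-state material and capsule size.
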(event Custom|EventLoadLevel
  (params (LevelsToLoad :type Array%20of%20Names) (LevelsToUnload :type Array%20of%20Names))
  (if (Utilities|Array|IsValidIndex LevelsToLoad (Variables|Default|GetCurLoadingLevel)) :!label _label
    (Game|LoadStreamLevel(byName) (Utilities|Array|Get(acopy) LevelsToLoad (Variables|Default|GetCurLoadingLevel)) true)
    (Math|Integer|IncrementInt (Variables|Default|GetCurLoadingLevel)
      (:%20%20
        (goto _label)))
    (else
      (Variables|Default|SetCurLoadingLevel 0)
      (if (Utilities|Array|IsValidIndex LevelsToUnload (Variables|Default|GetCurLoadingLevel)) :!label _label_2
        (Game|UnloadStreamLevel(byName) (Utilities|Array|Get(acopy) LevelsToUnload (Variables|Default|GetCurLoadingLevel)) false)
        (Math|Integer|IncrementInt (Variables|Default|GetCurLoadingLevel)
          (:%20%20
            (goto _label_2)))
        (else
          (Variables|Default|SetCurLoadingLevel 0))))))

(event EventBeginPlay
  (EventDispatchers|BindEventtoLoadLevels (delegate Custom|EventLoadLevel)))

(event Collision|EventActorBeginOverlap
  (params (OtherActor :type Actor%20Object%20Reference)))

(event EventTick
  (params (DeltaSeconds :type Float%20%28single-precision%29)))

(event EventInteract
  (params (Caller :type Character%20Object%20Reference))
  (CallFunction|DoAction Caller))

(fn ConstructionScript
  (bind _staticmesh (Variables|Default|GetStaticMesh))
  (bind _capsule (Variables|Default|GetCapsule))
  (if (Variables|Default|GetEnabled)
    (Rendering|Material|SetMaterial _staticmesh 0 (Variables|Default|GetEnabledMaterial))
    (else
      (Rendering|Material|SetMaterial _staticmesh 0 (Variables|Default|GetDisabledMaterial))))
  (Components|StaticMesh|SetStaticMesh (Variables|Default|GetStaticMesh) (Variables|Default|GetMesh))
  (Components|Capsule|SetCapsuleHalfHeight _capsule (Variables|Default|GetCapsuleHalfHeight) true)
  (Components|Capsule|SetCapsuleRadius _capsule (Variables|Default|GetCapsuleRadius) true))

(fn DoAction
  (params (Caller :type Character%20Object%20Reference))
  (if (Variables|Default|GetEnabled)
    (Default|CallLoadLevels (Variables|Default|GetLevelsToLoad) (Variables|Default|GetLevelsToUnload))
    (CallFunction|Disable)))

(fn Disable
  (Variables|Default|SetEnabled false)
  (Rendering|Material|SetMaterial (Variables|Default|GetStaticMesh) 0 (Variables|Default|GetDisabledMaterial)))