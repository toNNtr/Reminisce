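; InteractableToggler is a trigger actor that fires a list of interactables when a character overlaps its box.
; While Enabled, an overlap sends InteractMessage, with the character, to each Interactables entry implementing the Interactable interface.
; Enabled is set to the inverse of DoOnce before the Character cast, so with DoOnce on, any overlapping actor uses up the single trigger.
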(event OnComponentBeginOverlap(Box)
  (params (OverlappedComponent :type Primitive%20Component%20Object%20Reference) (OtherActor :type Actor%20Object%20Reference) (OtherComp :type Primitive%20Component%20Object%20Reference) (OtherBodyIndex :type Integer) (bFromSweep :type Boolean) (SweepResult :type Hit%20Result%20Structure%20%28by%20ref%29))
  (if (Variables|Default|GetEnabled)
    (Variables|Default|SetEnabled (not (Variables|Default|GetDoOnce)))
    (for _array_element (Variables|Default|GetInteractables)
      (if (Utilities|DoesObjectImplementInterface _array_element "/Game/Game/Blueprints/Interactable.Interactable_C")
        (bind _ascharacter (Utilities|Casting|CastToCharacter OtherActor))
        (Class|Interactable|Interact(Message) _array_element _ascharacter)))))

(event EventBeginPlay)

(event Collision|EventActorBeginOverlap
  (params (OtherActor :type Actor%20Object%20Reference)))

(event EventTick
  (params (DeltaSeconds :type Float%20%28single-precision%29)))

(fn ConstructionScript)