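; Scare-effect actor that flickers a streaming level's visibility when the player faces it after an interaction.
; Interact arms it, then Tick compares the player's forward vector with the direction to the actor via a dot-product threshold and fires the StartToggle dispatcher.
; Its bound handler waits, then runs a delay-driven loop that toggles visibility for the configured flashes, loading the level asynchronously if needed, and disarms afterward.
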(event Custom|CustomEvent_0
  (params (NewVisible :type Boolean))
  (bind _levelname (Variables|Default|GetLevelName))
  (bind _returnvalue (Class|GameplayStatics|GetStreamingLevel _levelname))
  (Variables|Default|SetToggling true)
  (Utilities|FlowControl|Delay (Variables|Default|GetDelay))
  (if (<= (Variables|Default|GetCurrentloop) (Variables|Default|GetFlashes)) :!label _label
    (Utilities|FlowControl|Delay (/ 1.0 (Math|Conversions|ToFloat(Integer) (Variables|Default|GetFlashingSpeed))))
    (if (and (not (Class|LevelStreaming|IsLevelLoaded _returnvalue)) (not (Variables|/Script/Engine.LevelStreaming|GetbShouldBeVisible _returnvalue)))
      (Game|LoadStreamLevel(byName) (Variables|Default|GetLevelName) false))
    (Variables|/Script/Engine.LevelStreaming|SetbShouldBeVisible _returnvalue (not (Variables|/Script/Engine.LevelStreaming|GetbShouldBeVisible _returnvalue)))
    (Math|Integer|IncrementInt (Variables|Default|GetCurrentloop)
      (:%20%20
        (goto _label)))
    (else
      (Variables|Default|SetCurrentloop 1)
      (Variables|Default|SetEnabled false)
      (Variables|Default|SetToggling false))))

(event EventBeginPlay
  (EventDispatchers|BindEventtoStartToggle (delegate Custom|CustomEvent_0)))

(event Collision|EventActorBeginOverlap
  (params (OtherActor :type Actor%20Object%20Reference)))

(event EventTick
  (params (DeltaSeconds :type Float%20%28single-precision%29))
  (if (and (not (Variables|Default|GetToggling)) (Variables|Default|GetEnabled))
    (bind _isfacing (CallFunction|IsPlayerFacingActor self (Variables|Default|GetAngle)))
    (if _isfacing
      (Default|CallStartToggle false))))

(event EventInteract
  (params (Caller :type Character%20Object%20Reference))
  (Variables|Default|SetEnabled true))

(fn ConstructionScript)

(fn IsPlayerFacingActor
  (params (Actor :type Actor%20Object%20Reference) (Angle :type Float%20%28single-precision%29))
  (bind _returnvalue (Game|GetPlayerCharacter 0))
  (return (>= (Math|Vector|DotProduct (Math|Vector|Normalize (- (Transformation|GetActorLocation Actor) (Transformation|GetActorLocation _returnvalue))) (Math|Vector|Normalize (Transformation|GetActorForwardVector _returnvalue))) Angle)))