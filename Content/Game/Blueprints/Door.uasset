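; Interactable door Blueprint that swings the Door component open or closed on each Interact, clockwise or counter-clockwise according to the Clockwise flag and OpenMaxDegree.
; Three timelines drive yaw by shortest-path lerping from the current rotation, each toggle stopping the opposing motion so it can reverse mid-swing.
; Any overlap with the Box component halts all timelines, freezing the door in place.
; The construction script pre-rotates doors that start Opened.
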(event OnComponentBeginOverlap(Box)
  (params (OverlappedComponent :type Primitive%20Component%20Object%20Reference) (OtherActor :type Actor%20Object%20Reference) (OtherComp :type Primitive%20Component%20Object%20Reference) (OtherBodyIndex :type Integer) (bFromSweep :type Boolean) (SweepResult :type Hit%20Result%20Structure%20%28by%20ref%29))
  (bind _door (Variables|Default|GetDoor))
  (bind _door_2 (Variables|Default|GetDoor))
  (bind _door_3 (Variables|Default|GetDoor))
  (Utilities|FlowControl|Sequence
    (:then_0
      (bind _alpha (Timeline|Timeline_1 Stop)
        (:Update
          (Transformation|SetRelativeRotation _door (Math|Rotator|Lerp(Rotator) (Variables|/Script/Engine.SceneComponent|GetRelativeRotation _door) (|MakeRot_3 0.0) _alpha true) false false))))
    (:then_1
      (bind _alpha_2 (Timeline|OpenClockwise Stop)
        (:Update
          (Transformation|SetRelativeRotation _door_2 (Math|Rotator|Lerp(Rotator) (Variables|/Script/Engine.SceneComponent|GetRelativeRotation _door_2) (|MakeRot (Variables|Default|GetOpenMaxDegree)) _alpha_2 true) false false))))
    (:then_2
      (bind _alpha_3 (Timeline|Timeline_0 Stop)
        (:Update
          (Transformation|SetRelativeRotation _door_3 (Math|Rotator|Lerp(Rotator) (Variables|/Script/Engine.SceneComponent|GetRelativeRotation _door_3) (|MakeRot_2 (- 3.6e+02 (Variables|Default|GetOpenMaxDegree))) _alpha_3 true) false false))))))

(event EventBeginPlay)

(event Collision|EventActorBeginOverlap
  (params (OtherActor :type Actor%20Object%20Reference)))

(event EventTick
  (params (DeltaSeconds :type Float%20%28single-precision%29)))

(event EventInteract
  (params (Caller :type Character%20Object%20Reference))
  (bind _door (Variables|Default|GetDoor))
  (bind _door_2 (Variables|Default|GetDoor))
  (bind _door_3 (Variables|Default|GetDoor))
  (if (Variables|Default|GetOpened)
    (Variables|Default|SetOpened false)
    (Utilities|FlowControl|Sequence
      (:then_0
        (bind _alpha (Timeline|OpenClockwise Stop)
          (:Update
            (Transformation|SetRelativeRotation _door_2 (Math|Rotator|Lerp(Rotator) (Variables|/Script/Engine.SceneComponent|GetRelativeRotation _door_2) (|MakeRot (Variables|Default|GetOpenMaxDegree)) _alpha true) false false))))
      (:then_1
        (bind _alpha_2 (Timeline|Timeline_0 Stop)
          (:Update
            (Transformation|SetRelativeRotation _door_3 (Math|Rotator|Lerp(Rotator) (Variables|/Script/Engine.SceneComponent|GetRelativeRotation _door_3) (|MakeRot_2 (- 3.6e+02 (Variables|Default|GetOpenMaxDegree))) _alpha_2 true) false false))))
      (:then_2
        (bind _alpha_3 (Timeline|Timeline_1 PlayFromStart)
          (:Update
            (Transformation|SetRelativeRotation _door (Math|Rotator|Lerp(Rotator) (Variables|/Script/Engine.SceneComponent|GetRelativeRotation _door) (|MakeRot_3 0.0) _alpha_3 true) false false)))))
    (else
      (Variables|Default|SetOpened true)
      (Utilities|FlowControl|Sequence
        (:then_0
          (Timeline|Timeline_1 Stop))
        (:then_1
          (if (Variables|Default|GetClockwise)
            (Timeline|OpenClockwise PlayFromStart)
            (else
              (Timeline|Timeline_0 PlayFromStart))))))))

(fn ConstructionScript
  (if (Variables|Default|GetOpened)
    (if (Variables|Default|GetClockwise)
      (Transformation|SetRelativeRotation (Variables|Default|GetDoor) (Math|Rotator|MakeRotator 0.0 0.0 (Variables|Default|GetOpenMaxDegree)) false false)
      (else
        (Transformation|SetRelativeRotation (Variables|Default|GetDoor) (Math|Rotator|MakeRotator 0.0 0.0 (- 3.6e+02 (Variables|Default|GetOpenMaxDegree))) false false)))))

(fn NewFunction0)